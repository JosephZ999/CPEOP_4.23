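; BP_Health is a health pickup that heals the player and removes itself when picked up.
; On BeginPlay, after the parent logic, it scales its Paper2D sprite linearly with its Value, so larger heals look bigger.
; The PickUp event checks that the player pawn is valid, adds Value to health through the pawn's HeroStats component, then destroys the actor.
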(event `self.ReceiveBeginPlay`
  (bind _returnvalue (+ (* (`self.Value`) 3.0) 3.0))
  (`parent.ReceiveBeginPlay`)
  (`SceneComponent.SetRelativeScale3D` (`self.PaperSprite`) (`KismetMathLibrary.MakeVector` _returnvalue _returnvalue _returnvalue)))

(event `self.PickUp`
  (bind _playerpawn (`self.PlayerPawn`))
  (`/Engine/EditorBlueprintResources/StandardMacros.IsValid` _playerpawn
    (:`Is Valid`
      (`HeroStats.AddHealth` (`self.GetComponentByClass` _playerpawn "/Script/CPEOP.HeroStats") (`self.Value`))
      (`self.K2_DestroyActor`))))

(fn `UserConstructionScript`
  (`parent.UserConstructionScript`))