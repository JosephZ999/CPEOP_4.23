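; BP_Power is a pickup that adds power to the player's hero stats.
; On BeginPlay it scales its paper sprite uniformly from its Value, so larger amounts appear bigger.
; When PickUp fires with a valid player pawn, it waits briefly, passes Value to AddPower on the pawn's HeroStats component, then destroys itself.
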(event `self.ReceiveBeginPlay`
  (bind _returnvalue (+ (* (`self.Value`) 4.0) 2.0))
  (`parent.ReceiveBeginPlay`)
  (`SceneComponent.SetRelativeScale3D` (`self.PaperSprite`) (`KismetMathLibrary.MakeVector` _returnvalue _returnvalue _returnvalue)))

(event `self.PickUp`
  (bind _playerpawn (`self.PlayerPawn`))
  (`/Engine/EditorBlueprintResources/StandardMacros.IsValid` _playerpawn
    (:`Is Valid`
      (`KismetSystemLibrary.Delay` 0.2)
      (`HeroStats.AddPower` (`self.GetComponentByClass` _playerpawn "/Script/CPEOP.HeroStats") (`self.Value`))
      (`self.K2_DestroyActor`))))

(fn `UserConstructionScript`
  (`parent.UserConstructionScript`))