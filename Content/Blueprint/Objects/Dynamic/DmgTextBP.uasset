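; DmgTextBP is a short-lived floating damage-number actor.
; On BeginPlay it passes the damage and crit values from its options to the DmgText widget in its widget component.
; It sets its projectile movement to drift slowly left or right along X based on MoveRight, then destroys itself after a brief delay.
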(event `self.ReceiveBeginPlay`
  (bind (_dmg _crit) (`self.getOptions`))
  (`|ExecutionSequence`
    (:`then_0`
      (bind _asdmg_text (cast `/Game/Blueprint/Objects/Dynamic/DmgText` (`WidgetComponent.GetUserWidgetObject` (`self.Widget`))))
      (`/Game/Blueprint/Objects/Dynamic/DmgText.Init` _asdmg_text _dmg _crit))
    (:`then_1`
      (`KismetSystemLibrary.Delay` 1.5)
      (`self.K2_DestroyActor`))
    (:`then_2`
      (set `MovementComponent.Velocity` (`KismetMathLibrary.MakeVector` (* 50.0 (select `bool` (`self.MoveRight`) :`false` -1.0 :`true` 1.0 :!type "Float (single-precision)")) 0.0 0.0) (`self.ProjectileMovement`)))))

(fn `UserConstructionScript`)