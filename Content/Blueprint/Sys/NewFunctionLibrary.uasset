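; Blueprint function library whose MyRandomVector picks an unobstructed random position along X on either side of a target location.
; Line traces run the given distance in +X and -X, and each clear trace yields a candidate at its end X, with random absolute Y and fixed Z.
; It picks randomly when both sides are clear, otherwise falls back to the first if clear, else the second, even if unset.
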(fn `MyRandomVector`
  (params (TargetLoc :type "Vector Structure") (dist :type "Float (double-precision)"))
  (returns (Out :type "Vector Structure"))
  (locals (FirstS :type Boolean) (SecondS :type Boolean) (Second :type "Vector Structure") (First :type "Vector Structure"))
  (bind _targetloc (`local.TargetLoc`))
  (bind _targetloc_2 (`local.TargetLoc`))
  (`|ExecutionSequence`
    (:`then_0`
      (bind (_outhit _returnvalue) (`KismetSystemLibrary.LineTraceSingle` null _targetloc_2 (+ _targetloc_2 (`KismetMathLibrary.MakeVector` dist)) "TraceTypeQuery4"))
      (if (not _returnvalue)
        (set `local.First` (`KismetMathLibrary.MakeVector` (.x (`.TraceEnd` (`GameplayStatics.BreakHitResult` _outhit))) (`KismetMathLibrary.RandomFloatInRange` -128.0 128.0) 50.0))
        (set `local.FirstS` true)))
    (:`then_1`
      (bind (_outhit_2 _returnvalue_2) (`KismetSystemLibrary.LineTraceSingle` null _targetloc (- _targetloc (`KismetMathLibrary.MakeVector` dist)) "TraceTypeQuery4"))
      (if (not _returnvalue_2)
        (set `local.Second` (`KismetMathLibrary.MakeVector` (.x (`.TraceEnd` (`GameplayStatics.BreakHitResult` _outhit_2))) (`KismetMathLibrary.RandomFloatInRange` -128.0 128.0) 50.0))
        (set `local.SecondS` true)))
    (:`then_2`
      ;[1 1 1] Select one
      (if (and (`local.FirstS`) (`local.SecondS`))
        (return (select `bool` (`KismetMathLibrary.RandomBool`) :`false` (`local.Second`) :`true` (`local.First`)))
        (elif (`local.FirstS`)
          (return (`local.First`))
          (else
            (return (`local.Second`))))))))