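; MyHud is a HUD Blueprint that manages the survival-mode player UI and relays health, mana and resource warnings to it.
; ShowGameUI lazily creates the SurvivalModeHUD widget, then adds or removes it from the viewport using a hidden flag.
; HP and MP updates restart timelines that ease displayed values toward targets by lerping from the last stored percentage.
; Without a valid widget, updates only store values, though UpdateMp writes into the HP variables.
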(event `self.ShowGameUI`
  (params (Hide :type Boolean))
  (`self.ShowPlayerUI` Hide))

(event `self.UpdateHp`
  (params (Hp :type "Float (single-precision)") (MaxHp :type "Float (single-precision)"))
  (bind _maxhp (`self.MaxHp`))
  (`/Engine/EditorBlueprintResources/StandardMacros.IsValid` (`self.PlayerUI`)
    (:`Is Valid`
      (set `self.MaxHp` MaxHp)
      (set `self.Hp` Hp)
      (bind (_direction _value) (`Timeline|HpCurve` :!via `PlayFromStart`)
        (:`Update`
          (bind _returnvalue (`KismetMathLibrary.Lerp` (* (`self.HpPercent`) (`self.MaxHp`)) (`self.Hp`) _value))
          (message `PlayerHUD.UpdateHp` (`self.PlayerUI`) _returnvalue _maxhp)
          (set `self.HpPercent` (/ _returnvalue _maxhp)))))
    (:`Is Not Valid`
      (set `self.MaxHp` MaxHp)
      (set `self.Hp` Hp))))

(event `self.UpdateMp`
  (params (Mp :type "Float (single-precision)") (MaxMp :type "Float (single-precision)"))
  (bind _maxmp (`self.MaxMp`))
  (`/Engine/EditorBlueprintResources/StandardMacros.IsValid` (`self.PlayerUI`)
    (:`Is Valid`
      (set `self.MaxMp` MaxMp)
      (set `self.Mp` Mp)
      (bind (_direction _value) (`Timeline|MpCurve` :!via `PlayFromStart`)
        (:`Update`
          (bind _returnvalue (`KismetMathLibrary.Lerp` (* (`self.MpPercent`) (`self.MaxMp`)) (`self.Mp`) _value))
          (message `PlayerHUD.UpdateMp` (`self.PlayerUI`) _returnvalue _maxmp)
          (set `self.MpPercent` (/ _returnvalue _maxmp)))))
    (:`Is Not Valid`
      (set `self.MaxHp` MaxMp)
      (set `self.Hp` Mp))))

(event `self.NotEnoughPower`
  (bind _playerui (`self.PlayerUI`))
  (`/Engine/EditorBlueprintResources/StandardMacros.IsValid` _playerui
    (:`Is Valid`
      (message `PlayerHUD.NotEnoughPower` _playerui))))

(event `self.NotEnoughStamina`
  (bind _playerui (`self.PlayerUI`))
  (`/Engine/EditorBlueprintResources/StandardMacros.IsValid` _playerui
    (:`Is Valid`
      (message `PlayerHUD.NotEnoughStamina` _playerui))))

(event `self.SkillActivated`)

(event `self.SkillDeactivated`)

(fn `ShowPlayerUI`
  (params (Hide :type Boolean))
  (if (not Hide)
    (`/Engine/EditorBlueprintResources/StandardMacros.IsValid` (`self.PlayerUI`)
      (:`Is Valid`
        (if (`self.PlayerUI_Hidden`)
          (`UserWidget.AddToViewport` (`self.PlayerUI`) 0 :!label _label)
          (set `self.PlayerUI_Hidden` false)))
      (:`Is Not Valid`
        (bind _returnvalue (`|CreateWidget` "/Game/Blueprint/UI/GameHuds/SurvivalModeHUD.SurvivalModeHUD_C"))
        (set `self.PlayerUI` _returnvalue)
        (goto _label)))
    (elif (not (`self.PlayerUI_Hidden`))
      (`/Engine/EditorBlueprintResources/StandardMacros.IsValid` (`self.PlayerUI`)
        (:`Is Valid`
          (`Widget.RemoveFromParent` (`self.PlayerUI`))
          (set `self.PlayerUI_Hidden` true))))))

(fn `UserConstructionScript`)