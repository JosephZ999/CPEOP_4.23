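; Game instance that manages menu widgets and persists achievements and progress.
; Init pre-creates the main, options and challenge menus hidden through a shared show/hide helper that writes cached references by ref.
; Achievements and indexed integers live in separate lazily loaded SaveGame slots; new achievement keys are saved and can trigger a reused notice widget, gated by a game mode check.
; DropItem returns a constant, while GiveItem and unlock functions are empty stubs.
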(event `self.ReceiveInit`
  (`self.SetMainMenu` true)
  (`self.SetOptionsMenu` true)
  (`self.SetChallengeMenu` true))

(fn `CheckAchievement`
  (params (Key :type Name))
  (returns (return :type Boolean))
  (bind _achievements_sobject (`self.Achievements_SObject`))
  (`/Engine/EditorBlueprintResources/StandardMacros.IsValid` (`self.Achievements_SObject`)
    (:`Is Valid`
      _)
    (:`Is Not Valid`
      (bind _loaded (`self.CreateSaveGameObj` (`self.AchivementSlot`) _achievements_sobject "/Game/Blueprint/Sys/SaveGame/BP_Achievements.BP_Achievements_C"))
      (if (and _loaded (`KismetSystemLibrary.IsValid` _achievements_sobject))
        _
        (else
          (return false)))))
  (for _array_element (`/Game/Blueprint/Sys/SaveGame/BP_Achievements.Kays` (`self.Achievements_SObject`))
    (if (== _array_element Key)
      (return true)))
  (return false))

(fn `CreateSaveGameObj`
  (params (Slot :type String) (Var :type "SaveGame Object Reference (by ref)") (Class :type "SaveGame Class Reference"))
  (returns (Loaded :type Boolean))
  (bind _returnvalue (`GameplayStatics.DoesSaveGameExist` (`local.Slot`)))
  (if _returnvalue
    (bind _returnvalue_2 (`GameplayStatics.LoadGameFromSlot` (`local.Slot`)))
    (`|VariableSetRef` (`local.Var`) _returnvalue_2)
    (return true)
    (else
      (bind _returnvalue_3 (`GameplayStatics.CreateSaveGameObject` (`local.Class`)))
      (`|VariableSetRef` (`local.Var`) _returnvalue_3)
      (`GameplayStatics.SaveGameToSlot` _returnvalue_3 (`local.Slot`))
      (return false))))

(fn `DropItem`
  (params (Hero :type "HeroBase Class Reference") (Items :type "Array of /Game/Blueprint/Objects/Items/ItemBase Class Reference"))
  (returns (DelayTime :type "Float (double-precision)"))
  (return 4.0))

(fn `GiveItem`)

(fn `LoadAchievements`
  (returns (Success :type Boolean) (Keys :type "Array of Name"))
  (bind _achievements_sobject (`self.Achievements_SObject`))
  (`/Engine/EditorBlueprintResources/StandardMacros.IsValid` _achievements_sobject
    (:`Is Valid`
      (return true (`/Game/Blueprint/Sys/SaveGame/BP_Achievements.Kays` _achievements_sobject)))
    (:`Is Not Valid`
      (bind _returnvalue (`GameplayStatics.DoesSaveGameExist` (`self.AchivementSlot`)))
      (if _returnvalue
        (bind _returnvalue_2 (`GameplayStatics.LoadGameFromSlot` (`self.AchivementSlot`)))
        (bind _asbp_achievements (cast `/Game/Blueprint/Sys/SaveGame/BP_Achievements` _returnvalue_2))
        (bind _output_get (set `self.Achievements_SObject` _asbp_achievements))
        (return true (`/Game/Blueprint/Sys/SaveGame/BP_Achievements.Kays` _output_get))
        (else
          (bind _returnvalue_3 (`GameplayStatics.CreateSaveGameObject` "/Game/Blueprint/Sys/SaveGame/BP_Achievements.BP_Achievements_C"))
          (set `self.Achievements_SObject` _returnvalue_3)
          (`GameplayStatics.SaveGameToSlot` (`self.Achievements_SObject`) (`self.AchivementSlot`))
          (return true (`|MakeArray` "None" :!type "Name")))))))

(fn `LoadInteger`
  (params (Index :type Name))
  (returns (Success :type Boolean) (Value :type Integer))
  (bind (_value _returnvalue) (`BlueprintMapLibrary.Map_Find` (`/Game/Blueprint/Sys/SaveGame/BP_Progress.Integer` (`self.Progress_Object`)) Index))
  (`|ExecutionSequence`
    (:`then_0`
      (`/Engine/EditorBlueprintResources/StandardMacros.IsValid` (`self.Progress_Object`)
        (:`Is Not Valid`
          (bind _returnvalue_2 (`GameplayStatics.DoesSaveGameExist` (`self.ProgressSlot`)))
          (if _returnvalue_2
            (bind _returnvalue_3 (`GameplayStatics.LoadGameFromSlot` (`self.ProgressSlot`)))
            (bind _asbp_progress (cast `/Game/Blueprint/Sys/SaveGame/BP_Progress` _returnvalue_3))
            (set `self.Progress_Object` _asbp_progress)
            (else
              (bind _returnvalue_4 (`GameplayStatics.CreateSaveGameObject` "/Game/Blueprint/Sys/SaveGame/BP_Progress.BP_Progress_C"))
              (set `self.Progress_Object` _returnvalue_4)
              (return false 0))))))
    (:`then_1`
      (if _returnvalue
        (return true _value)
        (else
          (return false 0))))))

(fn `SaveAchievement`
  (params (Key :type Name))
  (returns (Success :type Boolean))
  (`/Engine/EditorBlueprintResources/StandardMacros.IsValid` (`self.Achievements_SObject`)
    (:`Is Valid`
      (for _array_element (`/Game/Blueprint/Sys/SaveGame/BP_Achievements.Kays` (`self.Achievements_SObject`)) :!label _label
        (if (== _array_element Key)
          (return false))))
    (:`Is Not Valid`
      (bind _loaded (`self.CreateSaveGameObj` (`self.AchivementSlot`) (`self.Achievements_SObject`) "/Game/Blueprint/Sys/SaveGame/BP_Achievements.BP_Achievements_C"))
      (if _loaded
        (goto _label)
        (else
          _))))
  (`KismetArrayLibrary.Array_Add` (`/Game/Blueprint/Sys/SaveGame/BP_Achievements.Kays` (`self.Achievements_SObject`)) Key)
  (`GameplayStatics.SaveGameToSlot` (`self.Achievements_SObject`) (`self.AchivementSlot`))
  (`self.ShowNewAchievement` Key)
  (return true))

(fn `SaveInteger`
  (params (Index :type Name) (Value :type Integer))
  (returns (Success :type Boolean))
  (`|ExecutionSequence`
    (:`then_0`
      (`/Engine/EditorBlueprintResources/StandardMacros.IsValid` (`self.Progress_Object`)
        (:`Is Not Valid`
          (bind _returnvalue (`GameplayStatics.DoesSaveGameExist` (`self.ProgressSlot`)))
          (if _returnvalue
            (bind _returnvalue_2 (`GameplayStatics.LoadGameFromSlot` (`self.ProgressSlot`)))
            (bind _asbp_progress (cast `/Game/Blueprint/Sys/SaveGame/BP_Progress` _returnvalue_2))
            (set `self.Progress_Object` _asbp_progress)
            (else
              (bind _returnvalue_3 (`GameplayStatics.CreateSaveGameObject` "/Game/Blueprint/Sys/SaveGame/BP_Progress.BP_Progress_C"))
              (set `self.Progress_Object` _returnvalue_3))))))
    (:`then_1`
      (`BlueprintMapLibrary.Map_Add` (`/Game/Blueprint/Sys/SaveGame/BP_Progress.Integer` (`self.Progress_Object`)) Index Value)
      (bind _returnvalue_4 (`GameplayStatics.SaveGameToSlot` (`self.Progress_Object`) (`self.ProgressSlot`)))
      (return _returnvalue_4))))

(fn `SetChallengeMenu`
  (params (Hide :type Boolean))
  (locals (WidgetClass :type "UserWidget Class Reference" :default "WidgetBlueprintGeneratedClass'/Game/Blueprint/UI/Menu/1_Challenge.1_Challenge_C'"))
  (`self.ShowHideWidget` Hide (`self.W_Challenge`) (`local.WidgetClass`)))

(fn `SetMainMenu`
  (params (Hide :type Boolean))
  (locals (MainMenuClass :type "UserWidget Class Reference" :default "WidgetBlueprintGeneratedClass'/Game/Blueprint/UI/Menu/0_Main.0_Main_C'"))
  (`self.ShowHideWidget` (`local.Hide`) (`self.W_MainMenu`) (`local.MainMenuClass`)))

(fn `SetOptionsMenu`
  (params (Hide :type Boolean))
  (locals (W_OptionsClass :type "UserWidget Class Reference" :default "WidgetBlueprintGeneratedClass'/Game/Blueprint/UI/Menu/2_Options.2_Options_C'"))
  (`self.ShowHideWidget` (`local.Hide`) (`self.W_Options`) (`local.W_OptionsClass`)))

(fn `ShowHideWidget`
  (params (Hide :type Boolean) (WidgetRef :type "UserWidget Object Reference (by ref)") (ClassRef :type "UserWidget Class Reference"))
  (bind _classref (`local.ClassRef`))
  (bind _classref_2 (`local.ClassRef`))
  (bind _widgetref (`local.WidgetRef`))
  (if (not Hide)
    (`/Engine/EditorBlueprintResources/StandardMacros.IsValid` (`local.WidgetRef`)
      (:`Is Valid`
        (`UserWidget.AddToViewport` (`local.WidgetRef`) 0))
      (:`Is Not Valid`
        (if (`KismetSystemLibrary.IsValidClass` _classref)
          (bind _returnvalue (`|CreateWidget` _classref))
          (`|VariableSetRef` (`local.WidgetRef`) _returnvalue)
          (`UserWidget.AddToViewport` (`local.WidgetRef`) 0))))
    (else
      (`/Engine/EditorBlueprintResources/StandardMacros.IsValid` _widgetref
        (:`Is Valid`
          (`Widget.RemoveFromParent` _widgetref))
        (:`Is Not Valid`
          (if (`KismetSystemLibrary.IsValidClass` _classref_2)
            (bind _returnvalue_2 (`|CreateWidget` _classref_2))
            (`|VariableSetRef` (`local.WidgetRef`) _returnvalue_2)))))))

(fn `ShowNewAchievement`
  (params (Key :type Name))
  (bind _w_ach_ref (`self.W_Ach_Ref`))
  (bind _success (message `/Game/Blueprint/Sys/Interface/RefInterface.GetGameModeBP` (`GameplayStatics.GetGameMode`)))
  (if (not _success)
    (`/Engine/EditorBlueprintResources/StandardMacros.IsValid` _w_ach_ref
      (:`Is Valid`
        (`/Game/Blueprint/UI/Achievement/Ach_Notice.AddNew` _w_ach_ref (`local.Key`)))
      (:`Is Not Valid`
        (bind _returnvalue (`|CreateWidget` "/Game/Blueprint/UI/Achievement/Ach_Notice.Ach_Notice_C"))
        (`UserWidget.AddToViewport` _returnvalue 1)
        (`/Game/Blueprint/UI/Achievement/Ach_Notice.AddNew` _returnvalue (`local.Key`))
        (set `self.W_Ach_Ref` _returnvalue)))))

(fn `UnlockCharacter`)

(fn `UnlockSkill`)