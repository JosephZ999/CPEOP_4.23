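; Game mode that runs a match: it spawns and possesses the hero, spawns leveled team monsters with effects, and drops chance-based pickups.
; StartGame shows a get-ready widget, then after a delay enables player movement and starts a one-second looping game timer.
; Setter functions lazily create, cache and toggle loading, HUD and results widgets.
; It also binds to the controller's level-up event and provides a pausing level-up screen.
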(event `self.ReceiveBeginPlay`
  (bind _returnvalue (`GameplayStatics.GetPlayerController` 0))
  (set `PlayerController.bShowMouseCursor` true _returnvalue)
  (bind _asmy_player_controller_bp (cast `/Game/Blueprint/Sys/MyPlayerControllerBP` _returnvalue))
  (add `/Game/Blueprint/Sys/MyPlayerControllerBP.OnLevelUp` _asmy_player_controller_bp (`|CreateDelegate` :!event `HeroLevelUp`)))

(event `StartGame`
  (`|ExecutionSequence`
    (:`then_0`
      (`KismetSystemLibrary.Delay` 0.5)
      (bind _returnvalue (`|CreateWidget` "/Game/Blueprint/UI/Game/GetReadyWidget.GetReadyWidget_C"))
      (`UserWidget.AddToViewport` _returnvalue 0))
    (:`then_1`
      (`KismetSystemLibrary.Delay` 2.5)
      (`self.SetPlayerControl` true)
      (`self.SetGameTimer` false))))

(fn `CreateAHero`
  (params (Class :type "HeroBase Class Reference") (Location :type "Vector Structure") (Rotation :type "Rotator Structure"))
  (returns (Link :type "HeroBase Object Reference") (Success :type Boolean))
  (bind _returnvalue (`|SpawnActorFromClass` Class (`KismetMathLibrary.MakeTransform` Location Rotation) "Undefined" "OverrideRootScale" null null))
  (return _returnvalue (`KismetSystemLibrary.IsValid` _returnvalue)))

(fn `CreateAMonster`
  (params (Class :type "MonsterBase Class Reference") (Location :type "Vector Structure") (Rotation :type "Rotator Structure") (Team :type Byte) (level :type Byte))
  (returns (Success :type Boolean) (Monster :type "MonsterBase Object Reference"))
  (bind _returnvalue (`|SpawnActorFromClass` Class (`KismetMathLibrary.MakeTransform` Location Rotation) "AdjustIfPossibleButAlwaysSpawn" "OverrideRootScale" null null))
  (if (`KismetSystemLibrary.IsValid` _returnvalue)
    (set `UnitBase.Team` (+ Team 1) _returnvalue)
    (`MonsterStats.Init` (`MonsterBase.Stats` _returnvalue) (`local.level`))
    (`self.CreateSpawnEffect` (`self.K2_GetActorLocation` _returnvalue) (`MonsterBase.GetSpawnEffScale` _returnvalue))
    (return true _returnvalue)
    (else
      (return false null))))

(fn `CreatePickUpItems`
  (params (Item :type "/Game/Blueprint/Objects/Dynamic/PickUp/PickUpItemOptions Structure") (Location :type "Vector Structure"))
  (bind _returnvalue (`KismetMathLibrary.RandomFloatInRange` -25.0 25.0))
  (bind (_class _droprate _value) (break `/Game/Blueprint/Objects/Dynamic/PickUp/PickUpItemOptions` (`local.Item`)))
  (if (`KismetSystemLibrary.IsValidClass` _class)
    (if (`KismetMathLibrary.RandomBoolWithWeight` _droprate)
      (`|SpawnActorFromClass` _class (`KismetMathLibrary.MakeTransform` (`KismetMathLibrary.MakeVector` (+ (.x (`local.Location`)) _returnvalue) (.y (`local.Location`)) (+ (.z (`local.Location`)) _returnvalue)) (struct :`Roll` -20.0)) "Undefined" "OverrideRootScale" null _value null))))

(fn `CreateSpawnEffect`
  (params (Location :type "Vector Structure") (Scale :type "Float (double-precision)"))
  (`|SpawnActorFromClass` "/Game/Blueprint/Objects/Dynamic/MonsterSpawnEffect.MonsterSpawnEffect_C" (`KismetMathLibrary.MakeTransform` (`KismetMathLibrary.MakeVector` (.x (`local.Location`)) (+ (.y (`local.Location`)) 25.0)) (struct) (`KismetMathLibrary.MakeVector` Scale Scale Scale)) "AlwaysSpawn" "OverrideRootScale" null null)
  (return))

(fn `GetGameTime`
  (returns (GameTime :type Integer))
  (return (`self.GameTime`)))

(fn `HeroLevelUp`
  (locals (WidgetClass :type "UserWidget Class Reference"))
  (if (`KismetSystemLibrary.IsValidClass` (`self.W_LevelUpClass`))
    (bind _returnvalue (`|CreateWidget` (`self.W_LevelUpClass`)))
    (`UserWidget.AddToViewport` _returnvalue 0)
    (`GameplayStatics.SetGamePaused` true)
    (else
      (`/Game/Blueprint/Sys/MacroLibrary.DebugMessage` self "Level up widget is not selected"))))

(fn `Possess`
  (params (Hero :type "HeroBase Object Reference"))
  (bind _asmy_player_controller_bp (cast `/Game/Blueprint/Sys/MyPlayerControllerBP` (`GameplayStatics.GetPlayerController` 0)))
  (`Controller.Possess` _asmy_player_controller_bp (`local.Hero`))
  (`MyPlayerController.SetPlayerHero` _asmy_player_controller_bp (`local.Hero`))
  (set `self.PlayerCharacter` (`local.Hero`)))

(fn `SetCameraProjectionMode`
  (params (Perspective :type Boolean))
  (bind _playercharacter (`self.PlayerCharacter`))
  (bind _cameracomp (`HeroBase.CameraComp` _playercharacter))
  (if Perspective
    ;[1 1 1] Set Player Camera Options
    (`CameraComponent.SetProjectionMode` _cameracomp "Perspective")
    (`CameraComponent.SetFieldOfView` _cameracomp 10.0)
    (set `SpringArmComponent.TargetArmLength` 2500.0 (`HeroBase.ArmComp` _playercharacter))))

(fn `SetGameHud`
  (params (Show :type Boolean))
  (bind _w_gamehudclass (`self.W_GameHudClass`))
  (if Show
    (`/Engine/EditorBlueprintResources/StandardMacros.IsValid` (`self.W_GameHUD`)
      (:`Is Valid`
        (`UserWidget.AddToViewport` (`self.W_GameHUD`) 0))
      (:`Is Not Valid`
        (if (`KismetSystemLibrary.IsValidClass` _w_gamehudclass)
          (bind _returnvalue (`|CreateWidget` _w_gamehudclass))
          (bind _output_get (set `self.W_GameHUD` _returnvalue))
          (`UserWidget.AddToViewport` _output_get 0)
          (else
            (`/Game/Blueprint/Sys/MacroLibrary.DebugMessage` self "GameHUD class is not selected")))))
    (else
      (`/Engine/EditorBlueprintResources/StandardMacros.IsValid` (`self.W_GameHUD`)
        (:`Is Valid`
          (`Widget.RemoveFromParent` (`self.W_GameHUD`)))))))

(fn `SetGameResultsUI`
  (params (Show :type Boolean))
  (bind _w_resultsclass (`self.W_ResultsClass`))
  (if Show
    (`/Engine/EditorBlueprintResources/StandardMacros.IsValid` (`self.W_Results`)
      (:`Is Valid`
        (`UserWidget.AddToViewport` (`self.W_Results`) 0))
      (:`Is Not Valid`
        (if (`KismetSystemLibrary.IsValidClass` _w_resultsclass)
          (bind _returnvalue (`|CreateWidget` _w_resultsclass))
          (bind _output_get (set `self.W_Results` _returnvalue))
          (`UserWidget.AddToViewport` _output_get 0)
          (else
            (`/Game/Blueprint/Sys/MacroLibrary.DebugMessage` self "GameResults class is not selected")))))
    (else
      (`/Engine/EditorBlueprintResources/StandardMacros.IsValid` (`self.W_Results`)
        (:`Is Valid`
          (`Widget.RemoveFromParent` (`self.W_Results`)))))))

(fn `SetGameTimer`
  (params (Pause :type Boolean))
  (if (`KismetSystemLibrary.K2_IsValidTimerHandle` (`self.GameTimer`))
    (if Pause
      (`KismetSystemLibrary.K2_PauseTimerHandle` (`self.GameTimer`))
      (set `self.GameTimer` (struct)))
    (elif (not Pause)
      (bind _returnvalue (`KismetSystemLibrary.K2_SetTimer` null "TimeIncrement" 1.0 true 1.0))
      (set `self.GameTimer` _returnvalue)
      (set `self.GameTime` 0))))

(fn `SetLoadingScreen`
  (params (Show :type Boolean))
  (bind _w_loadingscreenclass (`self.W_LoadingScreenClass`))
  (if Show
    (`/Engine/EditorBlueprintResources/StandardMacros.IsValid` (`self.W_LoadingScreen`)
      (:`Is Valid`
        (`UserWidget.AddToViewport` (`self.W_LoadingScreen`) 3))
      (:`Is Not Valid`
        (if (`KismetSystemLibrary.IsValidClass` _w_loadingscreenclass)
          (bind _returnvalue (`|CreateWidget` _w_loadingscreenclass))
          (bind _output_get (set `self.W_LoadingScreen` _returnvalue))
          (`UserWidget.AddToViewport` _output_get 3)
          (else
            (`/Game/Blueprint/Sys/MacroLibrary.DebugMessage` self "LoadingScreen class is not selected")))))
    (else
      (`/Engine/EditorBlueprintResources/StandardMacros.IsValid` (`self.W_LoadingScreen`)
        (:`Is Valid`
          (`Widget.RemoveFromParent` (`self.W_LoadingScreen`)))))))

(fn `SetPlayerControl`
  (params (Enable :type Boolean))
  (bind _asmy_player_controller_bp (cast `/Game/Blueprint/Sys/MyPlayerControllerBP` (`GameplayStatics.GetPlayerController` 0)))
  (set `/Game/Blueprint/Sys/MyPlayerControllerBP.CanMove` Enable _asmy_player_controller_bp))

(fn `SetPlayerHUD`
  (params (Show :type Boolean))
  (bind _w_playerhudclass (`self.W_PlayerHudClass`))
  (bind (_asplayer_input _bsuccess) (cast `/Game/Blueprint/UI/GameHuds/PlayerInput` (`self.W_PlayerHUD`) :!pure true))
  (if Show
    (`/Engine/EditorBlueprintResources/StandardMacros.IsValid` (`self.W_PlayerHUD`)
      (:`Is Valid`
        (`UserWidget.AddToViewport` (`self.W_PlayerHUD`) 0))
      (:`Is Not Valid`
        (if (`KismetSystemLibrary.IsValidClass` _w_playerhudclass)
          (bind _returnvalue (`|CreateWidget` _w_playerhudclass))
          (set `self.W_PlayerHUD` _returnvalue)
          (bind _asmy_player_controller_bp (cast `/Game/Blueprint/Sys/MyPlayerControllerBP` (`GameplayStatics.GetPlayerController` 0)))
          (if _bsuccess
            (set `/Game/Blueprint/Sys/MyPlayerControllerBP.W_PlayerInput` _asplayer_input _asmy_player_controller_bp)
            (`UserWidget.AddToViewport` (`self.W_PlayerHUD`) 0))
          (else
            (`/Game/Blueprint/Sys/MacroLibrary.DebugMessage` self "PlayerHUD class is not selected")))))
    (else
      (`/Engine/EditorBlueprintResources/StandardMacros.IsValid` (`self.W_PlayerHUD`)
        (:`Is Valid`
          (`Widget.RemoveFromParent` (`self.W_PlayerHUD`)))))))

(fn `TimeIncrement`
  (`/Engine/EditorBlueprintResources/StandardMacros.IncrementInt` (`self.GameTime`)))

(fn `UserConstructionScript`)