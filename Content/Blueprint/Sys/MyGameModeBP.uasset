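; Game mode Blueprint that runs match start and finish and manages the game's UI, including versus and survival HUDs, loading screen, results and achievement notices.
; Start and finish extend parent events, toggling player control and input UI; start also caches the hero's same-team allies.
; Interface-style messages drive controller HUD updates and forward saves, loads and achievements to the game instance, queuing new achievement keys for display.
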(event `self.ReceiveBeginPlay`
  (set `PlayerController.bShowMouseCursor` true (`GameplayStatics.GetPlayerController` 0))
  (`KismetArrayLibrary.Array_Clear` (`self.NewAchievements`)))

(event `self.StartGame`
  (`parent.StartGame`)
  (`self.SetPlayerControl` true)
  (message `PlayerHUD.ShowInputUI` (`self.GetController`) false)
  (bind _allies (`self.FindAllies`))
  (set `self.Allies` _allies))

(event `self.FinishGame`
  (params (Title :type "Text (by ref)") (GameResult :type "EGameResultType Enum" :default "Win"))
  (`parent.FinishGame` Title GameResult)
  (`self.ShowGameResults` Title GameResult)
  (`self.SetPlayerControl` false)
  (message `PlayerHUD.ShowInputUI` (`self.GetController`) true)
  (`UnitBase.SetMoveVector` (`self.GetPlayerHero`) (0.0 0.0 0.0)))

(event `/Game/Blueprint/Sys/Interface/BP_PlayerHUD.CloseResultsWidget`
  ;[1 1 1] UI Interface
  (`GameplayStatics.OpenLevel` "Main"))

(event `/Game/Blueprint/Sys/Interface/BP_PlayerHUD.ShowNewAchievements`
  ;[1 1 1] UI Interface
  (if (> (`KismetArrayLibrary.Array_Length` (`self.NewAchievements`)) 0)
    (bind _returnvalue (`|CreateWidget` "/Game/Blueprint/UI/Achievement/Ach_Notice.Ach_Notice_C" null (`self.NewAchievements`)))
    (`UserWidget.AddToViewport` _returnvalue 1)))

(event `ShowGameHud_1`
  (params (Visible :type Boolean))
  (bind _returnvalue (`self.GetController`))
  (bind _returnvalue_2 (not Visible))
  ;[1 1 1] UI Interface
  (message `PlayerHUD.ShowGameUI` _returnvalue _returnvalue_2)
  (message `PlayerHUD.ShowInputUI` _returnvalue _returnvalue_2))

(event `self.ShowGameUI`
  (params (Hide :type Boolean))
  (bind _returnvalue (`self.GetController`))
  (bind _herostatscomp (`HeroBase.HeroStatsComp` (`self.GetPlayerHero`)))
  ;[1 1 1] UI Interface
  (message `PlayerHUD.ShowGameUI` (`self.GetController`) Hide)
  (if (not Hide)
    (message `PlayerHUD.UpdateHp` _returnvalue (`UnitStatsBase.GetHealth` _herostatscomp) (`UnitStatsBase.GetMaxHealth` _herostatscomp))
    (message `PlayerHUD.UpdateMp` _returnvalue (`HeroStats.GetPower` _herostatscomp) (`HeroStats.GetMaxPower` _herostatscomp))
    (message `PlayerHUD.UpdateExp` _returnvalue (`KismetMathLibrary.Conv_IntToDouble` (`HeroStats.GetExp` _herostatscomp)) (`KismetMathLibrary.Conv_IntToDouble` (`HeroStats.GetMaxExp` _herostatscomp)))
    (message `PlayerHUD.UpdateLevel` (`self.GetController`) (`HeroStats.GetLevel` _herostatscomp))))

(event `/Game/Blueprint/Sys/Interface/BP_PlayerHUD.ShowLoadingScreen`
  (params (Duration :type "Float (single-precision)"))
  (`self.SetLoadingScreen` true)
  (`KismetSystemLibrary.Delay` Duration)
  (`self.SetLoadingScreen` false))

(fn `BossHealth`
  (params (Boss :type "UnitBase Object Reference"))
  (message `/Game/Blueprint/Sys/Interface/BP_PlayerHUD.ShowBossHealth` (`self.W_VersusUI`) Boss))

(fn `CanShakeCamera`
  (params (OwnerUnit :type "Actor Object Reference") (DamagedUnit :type "Actor Object Reference"))
  (returns (ReturnValue :type Boolean))
  (bind _returnvalue (`self.GetPlayerHero`))
  (return (or (== OwnerUnit _returnvalue) (== DamagedUnit _returnvalue))))

(fn `CheckAchievement`
  (params (Key :type Name))
  (returns (return :type Boolean))
  (return false))

(fn `FindAllies`
  (returns (Allies :type "Array of UnitBase Object Reference"))
  (locals (LocArray :type "Array of UnitBase Object Reference"))
  (bind _returnvalue (`self.GetPlayerHero`))
  (`KismetArrayLibrary.Array_Clear` (`local.LocArray`))
  (bind _outactors (`GameplayStatics.GetAllActorsOfClass` "/Script/CPEOP.UnitBase"))
  (for _array_element _outactors
    (if (and (== (`UnitBase.Team` _array_element) (`UnitBase.Team` _returnvalue)) (!= _array_element _returnvalue))
      (`KismetArrayLibrary.Array_Add` (`local.LocArray`) _array_element)))
  (return (`local.LocArray`)))

(fn `GetAllAllies`
  (returns (Units :type "Array of UnitBase Object Reference"))
  (locals (LocArray :type "Array of UnitBase Object Reference"))
  (return (`self.Allies`)))

(fn `GetGameModeBP`
  (returns (Success :type Boolean) (Ref :type "/Game/Blueprint/Sys/MyGameModeBP Object Reference"))
  (return true self))

(fn `LoadAchievements`
  (returns (Success :type Boolean) (Keys :type "Array of Name"))
  (return false))

(fn `LoadInt`
  (params (Key :type Name))
  (returns (Success :type Boolean) (Value :type Integer))
  (bind (_success _value) (message `/Game/Blueprint/Sys/Interface/SaveLoad.LoadInteger` (`GameplayStatics.GetGameInstance`) Key))
  (return _success _value))

(fn `LoadInteger`
  (params (Index :type Name))
  (returns (Success :type Boolean) (Value :type Integer))
  (return false 0))

(fn `NewAchievement`
  (params (Key :type Name))
  (bind _success (message `/Game/Blueprint/Sys/Interface/SaveLoad.SaveAchievement` (`GameplayStatics.GetGameInstance`) Key))
  (if _success
    (`KismetArrayLibrary.Array_Add` (`self.NewAchievements`) (`local.Key`))))

(fn `SaveAchievement`
  (params (Key :type Name))
  (returns (Success :type Boolean))
  (return false))

(fn `SaveInt`
  (params (Key :type Name) (valeu :type Integer))
  (returns (Success :type Boolean))
  (bind _success (message `/Game/Blueprint/Sys/Interface/SaveLoad.SaveInteger` (`GameplayStatics.GetGameInstance`) Key valeu))
  (return _success))

(fn `SaveInteger`
  (params (Index :type Name) (Value :type Integer))
  (returns (Success :type Boolean))
  (return false))

(fn `SetCameraProjectionMode`
  (params (Perspective :type Boolean))
  (bind _returnvalue (`self.GetPlayerHero`))
  (bind _cameracomp (`HeroBase.CameraComp` _returnvalue))
  (if Perspective
    ;[1 1 1] Set Player Camera Options
    (`CameraComponent.SetProjectionMode` _cameracomp "Perspective")
    (`CameraComponent.SetFieldOfView` _cameracomp 20.0)
    (set `SpringArmComponent.TargetArmLength` 1400.0 (`HeroBase.ArmComp` _returnvalue))))

(fn `SetGameResultsUI`
  (params (Show :type Boolean))
  (bind _w_resultsclass (`self.W_ResultsClass`))
  (if Show
    (`/Engine/EditorBlueprintResources/StandardMacros.IsValid` (`self.W_Results`)
      (:`Is Valid`
        (`UserWidget.AddToViewport` (`self.W_Results`) 0))
      (:`Is Not Valid`
        (if (`KismetSystemLibrary.IsValidClass` _w_resultsclass)
          (bind _returnvalue (`|CreateWidget` _w_resultsclass))
          (bind _output_get (set `self.W_Results` _returnvalue))
          (`UserWidget.AddToViewport` _output_get 0)
          (else
            (`/Game/Blueprint/Sys/MacroLibrary.DebugMessage` self "GameResults class is not selected")))))
    (else
      (`/Engine/EditorBlueprintResources/StandardMacros.IsValid` (`self.W_Results`)
        (:`Is Valid`
          (`Widget.RemoveFromParent` (`self.W_Results`)))))))

(fn `SetLoadingScreen`
  (params (Show :type Boolean))
  (bind _w_loadingscreenclass (`self.W_LoadingScreenClass`))
  (if Show
    (`/Engine/EditorBlueprintResources/StandardMacros.IsValid` (`self.W_LoadingScreen`)
      (:`Is Valid`
        (`UserWidget.AddToViewport` (`self.W_LoadingScreen`) 3))
      (:`Is Not Valid`
        (if (`KismetSystemLibrary.IsValidClass` _w_loadingscreenclass)
          (bind _returnvalue (`|CreateWidget` _w_loadingscreenclass))
          (bind _output_get (set `self.W_LoadingScreen` _returnvalue))
          (`UserWidget.AddToViewport` _output_get 3)
          (else
            (`/Game/Blueprint/Sys/MacroLibrary.DebugMessage` self "LoadingScreen class is not selected")))))
    (else
      (`/Engine/EditorBlueprintResources/StandardMacros.IsValid` (`self.W_LoadingScreen`)
        (:`Is Valid`
          (`Widget.RemoveFromParent` (`self.W_LoadingScreen`)))))))

(fn `SetPlayerControl`
  (params (Enable :type Boolean))
  (bind _asmy_player_controller_bp (cast `/Game/Blueprint/Sys/MyPlayerControllerBP` (`GameplayStatics.GetPlayerController` 0)))
  (set `/Game/Blueprint/Sys/MyPlayerControllerBP.CanMove` Enable _asmy_player_controller_bp))

(fn `ShowGameResults`
  (params (Title :type Text) (State :type "EGameResultType Enum" :default "Win"))
  (bind _returnvalue (`|CreateWidget` "/Game/Blueprint/UI/Game/BattleResult.BattleResult_C"))
  (`|ExecutionSequence`
    (:`then_0`
      (set `/Game/Blueprint/UI/Game/BattleResult.Title` Title _returnvalue)
      (set `/Game/Blueprint/UI/Game/BattleResult.Time` (`self.GetGameTime`) _returnvalue)
      (set `/Game/Blueprint/UI/Game/BattleResult.Kills` (`self.GetPlayerKills`) _returnvalue))
    (:`then_1`
      (`UserWidget.AddToViewport` _returnvalue 0))))

(fn `ShowReadyAnim`
  (locals (WidgetClass :type "UserWidget Class Reference" :default "WidgetBlueprintGeneratedClass'/Game/Blueprint/UI/Game/GetReadyWidget.GetReadyWidget_C'"))
  (bind _returnvalue (`|CreateWidget` (`local.WidgetClass`)))
  (`UserWidget.AddToViewport` _returnvalue 0))

(fn `ShowSurvivalUI`
  (params (Hide :type Boolean))
  (if (not Hide)
    (`/Engine/EditorBlueprintResources/StandardMacros.IsValid` (`self.W_Results`)
      (:`Is Valid`
        (`UserWidget.AddToViewport` (`self.W_Results`) 0))
      (:`Is Not Valid`
        (bind _returnvalue (`|CreateWidget` "/Game/Blueprint/UI/GameHuds/SurvivalModeHUD.SurvivalModeHUD_C"))
        (bind _output_get (set `self.W_SurvivalUI` _returnvalue))
        (`UserWidget.AddToViewport` _output_get 0)))
    (else
      (`/Engine/EditorBlueprintResources/StandardMacros.IsValid` (`self.W_Results`)
        (:`Is Valid`
          (`Widget.RemoveFromParent` (`self.W_Results`)))))))

(fn `ShowVersusUI`
  (params (Hide :type Boolean) (PlayerHero :type "HeroBase Object Reference") (EnemyHero :type "HeroBase Object Reference"))
  (bind _w_versusui (`self.W_VersusUI`))
  (if (not Hide)
    (`/Engine/EditorBlueprintResources/StandardMacros.IsValid` (`self.W_VersusUI`)
      (:`Is Valid`
        (set `/Game/Blueprint/UI/GameHuds/VersusModeHUD.PlayerHero` (`local.PlayerHero`) _w_versusui)
        (set `/Game/Blueprint/UI/GameHuds/VersusModeHUD.EnemyHero` (`local.EnemyHero`) _w_versusui))
      (:`Is Not Valid`
        (bind _returnvalue (`|CreateWidget` "/Game/Blueprint/UI/GameHuds/VersusModeHUD.VersusModeHUD_C" null PlayerHero EnemyHero))
        (bind _output_get (set `self.W_VersusUI` _returnvalue))))
    (`UserWidget.AddToViewport` _output_get 0)
    (else
      (`/Engine/EditorBlueprintResources/StandardMacros.IsValid` (`self.W_VersusUI`)
        (:`Is Valid`
          (`Widget.RemoveFromParent` (`self.W_VersusUI`)))))))

(fn `UserConstructionScript`)