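; Player controller that relays player input to the pawn and forwards gameplay UI updates to the HUD.
; Movement, action, dash and teleport events go to player pawn 0 as message calls, with axis movement gated by CanMove and IsKeyboardEnabled.
; Space teleports, while Tab or Android Back asks the game instance to pause when CanMove is set.
; HUD events pass visibility, stats, skill state and shortage warnings through as messages.
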(event `self.BtnSetMovement`
  (params (Value :type "Vector Structure"))
  ;[1 1 1] Hero Commands
  (message `HeroInput.BtnSetMovement` (`GameplayStatics.GetPlayerPawn` 0) Value))

(event `MoveCharacter`
  (params (Vec :type "Vector Structure"))
  ;[1 1 1] Player Input's Implementation
  (`self.BtnSetMovement` Vec))

(event `self.BtnAction`
  (params (action :type "EInputActionType Enum" :default "A_None") (btnReleased :type Boolean))
  ;[1 1 1] Hero Commands
  (message `HeroInput.BtnAction` (`GameplayStatics.GetPlayerPawn` 0) action btnReleased))

(event `Key|SpaceBar`
  (params (Key :type "Key Structure"))
  ;[1 1 1] Player Input's Implementation
  (:`Pressed`
    (`self.BtnTeleport`)))

(event `self.BtnDash`
  (params (forwardVector :type "Vector Structure") (Released :type Boolean))
  ;[1 1 1] Hero Commands
  (message `HeroInput.BtnDash` (`GameplayStatics.GetPlayerPawn` 0) forwardVector Released))

(event `self.BtnTeleport`
  ;[1 1 1] Hero Commands
  (message `HeroInput.BtnTeleport` (`GameplayStatics.GetPlayerPawn` 0)))

(event `InputAxis|MoveForward`
  (params (AxisValue :type "Float (single-precision)"))
  (if (and (`self.CanMove`) (`self.IsKeyboardEnabled`))
    (`self.MoveCharacter` (`KismetMathLibrary.MakeVector` (`self.GetInputAxisValue`) (`self.GetInputAxisValue`)))))

(event `Key|Tab` :paused true
  (params (Key :type "Key Structure"))
  (:`Pressed`
    (if (`self.CanMove`) :!label _label
      (message `GameIns.PauseGame` (`GameplayStatics.GetGameInstance`)))))

(event `Key|Android_Back` :paused true
  (params (Key :type "Key Structure"))
  (:`Released`
    (goto _label)))

(event `self.ShowGameUI`
  (params (Hide :type Boolean))
  ;[1 1 1 0.5] HUD
  (message `PlayerHUD.ShowGameUI` (`self.GetHUD`) Hide))

(event `self.ShowInputUI`
  (params (Hide :type Boolean))
  ;[1 1 1 0.5] HUD
  (message `PlayerHUD.ShowInputUI` (`self.GetHUD`) Hide))

(event `self.ShowWarningNotice`
  (params (Hide :type Boolean))
  ;[1 1 1 0.5] HUD
  (message `PlayerHUD.ShowWarningNotice` (`self.GetHUD`) Hide))

(event `self.UpdateHp`
  (params (Hp :type "Float (single-precision)") (MaxHp :type "Float (single-precision)"))
  ;[1 1 1 0.5] HUD
  (message `PlayerHUD.UpdateHp` (`self.GetHUD`) Hp MaxHp))

(event `self.NotEnoughPower`
  ;[1 1 1 0.5] HUD
  (message `PlayerHUD.NotEnoughPower` (`self.GetHUD`)))

(event `self.UpdateLevel`
  (params (Level :type Byte))
  ;[1 1 1 0.5] HUD
  (message `PlayerHUD.UpdateLevel` (`self.GetHUD`) Level))

(event `self.NotEnoughStamina`
  ;[1 1 1 0.5] HUD
  (message `PlayerHUD.NotEnoughStamina` (`self.GetHUD`)))

(event `self.UpdateMp`
  (params (Mp :type "Float (single-precision)") (MaxMp :type "Float (single-precision)"))
  ;[1 1 1 0.5] HUD
  (message `PlayerHUD.UpdateMp` (`self.GetHUD`) Mp MaxMp))

(event `self.SkillActivated`
  ;[1 1 1 0.5] HUD
  (message `PlayerHUD.SkillActivated` (`self.GetHUD`)))

(event `self.UpdateExp`
  (params (Exp :type "Float (single-precision)") (MaxExp :type "Float (single-precision)"))
  ;[1 1 1 0.5] HUD
  (message `PlayerHUD.UpdateExp` (`self.GetHUD`) Exp MaxExp))

(event `self.SkillDeactivated`
  ;[1 1 1 0.5] HUD
  (message `PlayerHUD.SkillDeactivated` (`self.GetHUD`)))

(fn `UserConstructionScript`)