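; Ogichi character Blueprint that exposes start and stop controls for its AI.
; StartAI casts the possessing controller to OgichiAI, caches it and starts its AI with a fixed short time argument.
; StopAI, if that cached controller is valid, stops the AI, resets keys and zeroes the move vector.
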(event `self.StartAI`
  (bind _asogichi_ai (cast `OgichiAI` (`AIBlueprintHelperLibrary.GetAIController` self)))
  (bind _output_get (set `self.AiController` _asogichi_ai))
  (`UnitAIBase.StartAI` _output_get 0.2))

(event `self.StopAI`
  (`/Engine/EditorBlueprintResources/StandardMacros.IsValid` (`self.AiController`)
    (:`Is Valid`
      (`UnitAIBase.StopAI` (`self.AiController`))
      (`self.resetKeys`)
      (`self.SetMoveVector` (0.0 0.0 0.0)))))

(fn `UserConstructionScript`)