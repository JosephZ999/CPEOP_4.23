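; Ichigo hero character Blueprint that relays resource and skill state events to the game mode.
; Not-enough-power and not-enough-stamina events trigger their matching game mode messages, while skill activation and deactivation send a skill-changed message with a true or false flag.
; A HeroUsedBankai function reports the IsUsedBankai state, and the construction script is empty.
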(event `self.NotEnoughPower`
  (message `/Game/Blueprint/Sys/Interface/HudInterface.NotEnoughPower` (`GameplayStatics.GetGameMode`)))

(event `self.NotEnoughStamina`
  (message `/Game/Blueprint/Sys/Interface/HudInterface.NotEnoughStamina` (`GameplayStatics.GetGameMode`)))

(event `self.HeroSkillActivated`
  (message `/Game/Blueprint/Sys/Interface/HudInterface.OnSkillChanged` (`GameplayStatics.GetGameMode`) true))

(event `self.HeroSkillDeactivated`
  (message `/Game/Blueprint/Sys/Interface/HudInterface.OnSkillChanged` (`GameplayStatics.GetGameMode`) false))

(fn `HeroUsedBankai`
  (returns (value :type Boolean))
  (return (`self.IsUsedBankai`)))

(fn `UserConstructionScript`)