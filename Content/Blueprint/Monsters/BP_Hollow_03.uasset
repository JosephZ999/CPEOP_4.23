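; BP_Hollow_03 is a melee Hollow monster Blueprint driven by the HollowAI_1 controller.
; On StartAI it casts its AI controller, passes melee type, horizontal distance range and attack velocity parameters, then starts the AI.
; Tick only calls the parent, and a disconnected debug switch that prints the base movement state never runs.
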(event `self.ReceiveTick`
  (params (DeltaSeconds :type "Float (single-precision)"))
  (`parent.ReceiveTick` DeltaSeconds))

(event `self.StartAI`
  (bind _ashollow_ai_1 (cast `HollowAI_1` (`AIBlueprintHelperLibrary.GetAIController` self)))
  (`HollowAI_1.InitParams` _ashollow_ai_1 "Melee" 70.0 100.0 0.2)
  (`UnitAIBase.StartAI` _ashollow_ai_1 1.0))

(fn `UserConstructionScript`)